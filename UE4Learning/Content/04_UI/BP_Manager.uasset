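; BP_Manager runs a timed shape-spawning game, acting as the view target, creating WBP_UI and keeping a Count that can be incremented.
; While Duration remains, Tick spawns a BP_S every half second at a random point within SpawnArea.
; Each spawn gets a manager reference, a random mesh from four shapes and a random color through a dynamic material instance.
; BP_S actors that begin overlapping DestroyArea are destroyed.
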(event `self.ReceiveBeginPlay`
  (`PlayerController.SetViewTargetWithBlend` (`GameplayStatics.GetPlayerController` 0) self 0.0 "VTBlend_Linear" 0.0 false)
  (bind _returnvalue (`|CreateWidget` "/Game/04_UI/WBP_UI.WBP_UI_C"))
  (set `/Game/04_UI/WBP_UI.ManagerRef` self _returnvalue)
  (`UserWidget.AddToViewport` _returnvalue 0))

(event `self.ReceiveTick`
  (params (DeltaSeconds :type "Float (single-precision)"))
  (bind _returnvalue (`GameplayStatics.GetWorldDeltaSeconds`))
  (bind _output_get (set `self.Duration` (- (`self.Duration`) _returnvalue)))
  (if (> _output_get 0.0)
    (bind _output_get_2 (set `self.TimeBetweenSpawns` (- (`self.TimeBetweenSpawns`) _returnvalue)))
    (if (<= _output_get_2 0.0)
      (set `self.TimeBetweenSpawns` 0.5)
      (`self.SpawnObject`))))

(event `self.DestroyArea.OnComponentBeginOverlap`
  (params (OverlappedComponent :type "PrimitiveComponent Object Reference") (OtherActor :type "Actor Object Reference") (OtherComp :type "PrimitiveComponent Object Reference") (OtherBodyIndex :type Integer) (bFromSweep :type Boolean) (SweepResult :type "HitResult Structure (by ref)"))
  (bind _asbp_s (cast `/Game/04_UI/BP_S` OtherActor))
  (`self.K2_DestroyActor` _asbp_s))

(fn `CountIncrement`
  (`/Engine/EditorBlueprintResources/StandardMacros.IncrementInt` (`self.Count`)))

(fn `SpawnObject`
  (bind (_origin _boxextent) (`KismetSystemLibrary.GetComponentBounds` (`self.SpawnArea`)))
  (bind _returnvalue (`|SpawnActorFromClass` "/Game/04_UI/BP_S.BP_S_C" (`KismetMathLibrary.MakeTransform` (`KismetMathLibrary.RandomPointInBoundingBox` _origin _boxextent)) "Undefined" "OverrideRootScale" null null))
  (set `/Game/04_UI/BP_S.ManagerRef` self _returnvalue)
  (bind _staticmesh (`/Game/04_UI/BP_S.StaticMesh` _returnvalue))
  (`StaticMeshComponent.SetStaticMesh` _staticmesh (select `int` (`KismetMathLibrary.RandomIntegerInRange` 0 3) :`0` "/Game/04_UI/GeometryCatcher/Meshes/SM_Circle.SM_Circle" :`1` "/Game/04_UI/GeometryCatcher/Meshes/SM_Pentagon.SM_Pentagon" :`2` "/Game/04_UI/GeometryCatcher/Meshes/SM_Square.SM_Square" :`3` "/Game/04_UI/GeometryCatcher/Meshes/SM_Triangle.SM_Triangle" :!type "StaticMesh Object Reference"))
  (bind _returnvalue_2 (`PrimitiveComponent.CreateDynamicMaterialInstance` _staticmesh 0 "/Game/04_UI/GeometryCatcher/Materials/M_Base.M_Base"))
  (`MaterialInstanceDynamic.SetVectorParameterValue` _returnvalue_2 "Color" (select `int` (`KismetMathLibrary.RandomIntegerInRange` 0 4) :`0` (struct :`R` 0.846873 :`G` 0.01033 :`A` 1.0) :`1` (struct :`R` 0.03875 :`G` 0.607378 :`B` 0.775 :`A` 1.0) :`2` (struct :`R` 0.116875 :`G` 0.134935 :`B` 0.779167 :`A` 1.0) :`3` (struct :`R` 0.870833 :`G` 0.184984 :`B` 0.574895 :`A` 1.0) :`4` (struct :`R` 0.9 :`G` 0.747828 :`B` 0.235602 :`A` 1.0) :!type "LinearColor Structure")))

(fn `UserConstructionScript`)